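; BP_Ball is a physics ball for a game against an AI rival, apparently Pong-style.
; On BeginPlay it registers itself with BP_AIRival and launches its Sphere with a random sideways impulse, toward the Y direction chosen by Switch.
; Each hit raises BallSpeed, clamps the velocity to exactly that magnitude while keeping its direction, and prints it for debugging.
; When destroyed, it has BallSpawnerRef spawn another ball.
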(event EventBeginPlay
  (bind _returnvalue (Actor|GetActorOfClass "/Game/Blueprints/BP_AIRival.BP_AIRival_C"))
  (bind _output_get (Variables|Default|SetAIRivalRef _returnvalue))
  (Variables|/Game/Blueprints/BP_AIRival.BP_AIRival_C|SetBallRef _output_get self)
  (if (Variables|Default|GetSwitch?)
    (Physics|AddImpulse (Variables|Default|GetSphere) (Math|Vector|MakeVector (Math|Conversions|ToFloat(Integer) (Math|Random|RandomIntegerinRange -360 360)) 1e+03 0.0) "None" true)
    (else
      (Physics|AddImpulse (Variables|Default|GetSphere) (Math|Vector|MakeVector (Math|Conversions|ToFloat(Integer) (Math|Random|RandomIntegerinRange -360 360)) -1e+03 0.0) "None" true))))

(event Collision|EventHit
  (params (MyComp :type Primitive%20Component%20Object%20Reference) (Other :type Actor%20Object%20Reference) (OtherComp :type Primitive%20Component%20Object%20Reference) (bSelfMoved :type Boolean) (HitLocation :type Vector :default "0, 0, 0") (HitNormal :type Vector :default "0, 0, 0") (NormalImpulse :type Vector :default "0, 0, 0") (Hit :type Hit%20Result%20Structure%20%28by%20ref%29))
  (Variables|Default|SetBallSpeed (+ (Variables|Default|GetBallSpeed) 3e+01))
  (bind _returnvalue (Physics|GetPhysicsLinearVelocity (Variables|Default|GetSphere) "None"))
  (Physics|SetPhysicsLinearVelocity (Variables|Default|GetSphere) (Math|Vector|ClampVectorSize _returnvalue (Variables|Default|GetBallSpeed) (Variables|Default|GetBallSpeed)) false "None")
  (bind _returnvalue_2 (Physics|GetPhysicsLinearVelocity (Variables|Default|GetSphere) "None"))
  (Development|PrintString (Utilities|String|ToString(Vector) _returnvalue_2)))

(event EventDestroyed
  (Default|SpawnBall (Variables|Default|GetBallSpawnerRef)))

(fn ConstructionScript)