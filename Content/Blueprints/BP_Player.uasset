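; BP_Player is the player-controlled paddle in what the input context name indicates is a Pong-style game.
; On BeginPlay it adds the IMC_PinPong Enhanced Input mapping context, then creates a W_Score widget, stores it as ScoreHUD and adds it to the viewport.
; The IA_Movement action moves the Cube component along local X by input times Velocity, using a swept offset with no delta-time scaling.
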(event Input|EnhancedActionEvents|EnhancedInputActionIA_Movement
  (params (ActionValue :type Float%20%28double-precision%29) (ElapsedSeconds :type Float%20%28double-precision%29) (TriggeredSeconds :type Float%20%28double-precision%29) (InputAction :type Input%20Action%20Object%20Reference :default "/Game/Inputs/IA_Movement.IA_Movement"))
  (Transformation|AddLocalOffset (Variables|Default|GetCube) (Math|Vector|MakeVector (* ActionValue (Variables|Default|GetVelocity)) 0.0 0.0) true false))

(event EventBeginPlay
  (bind _asplayer_controller (Utilities|Casting|CastToPlayerController (Pawn|GetController)))
  (Utilities|IsValid (PlayerController|LocalPlayerSubsystems|GetEnhancedInputLocalPlayerSubsystem _asplayer_controller)
    (:Is%20Valid
      (Input|AddMappingContext (PlayerController|LocalPlayerSubsystems|GetEnhancedInputLocalPlayerSubsystem _asplayer_controller) "/Game/Inputs/IMC_PinPong.IMC_PinPong" 0 "(bIgnoreAllPressedKeysUntilRelease=True,bForceImmediately=False,bNotifyUserSettings=False)")
      (bind _returnvalue (UserInterface|CreateWidget "/Game/Blueprints/Widgets/W_Score.W_Score_C"))
      (bind _output_get (Variables|Default|SetScoreHUD _returnvalue))
      (UserInterface|Viewport|AddtoViewport _output_get 0))))

(fn ConstructionScript)