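; BP_Goal is a goal trigger that scores a point when a BP_Ball enters its box.
; On BeginPlay it caches the player pawn as BP_Player.
; On overlap, the PlayerGoal flag picks whether the player's ScoreHUD updates the player or AI rival score, then the ball is destroyed.
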(event OnComponentBeginOverlap(Box)
  (params (OverlappedComponent :type Primitive%20Component%20Object%20Reference) (OtherActor :type Actor%20Object%20Reference) (OtherComp :type Primitive%20Component%20Object%20Reference) (OtherBodyIndex :type Integer) (bFromSweep :type Boolean) (SweepResult :type Hit%20Result%20Structure%20%28by%20ref%29))
  (bind _asbp_ball (Utilities|Casting|CastToBP_Ball OtherActor))
  (if (Variables|Default|GetPlayerGoal?)
    (Default|UpdatePlayerScore (Variables|/Game/Blueprints/BP_Player.BP_Player_C|GetScoreHUD (Variables|Default|GetPlayerRef)))
    (else
      (Default|UpdateAIRivalScore (Variables|/Game/Blueprints/BP_Player.BP_Player_C|GetScoreHUD (Variables|Default|GetPlayerRef)))))
  (Actor|DestroyActor _asbp_ball))

(event EventBeginPlay
  (bind _asbp_player (Utilities|Casting|CastToBP_Player (Game|Player|GetPlayerPawn 0)))
  (Variables|Default|SetPlayerRef _asbp_player))

(fn ConstructionScript)